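; BP_ChatGPTAgent_Narrator is a GPT chat agent that generates five-member team tactics for a shooter map.
; On BeginPlay it seeds the message history with a system prompt built from MapDetails' image URL and color-to-zone list.
; SendGptMessage appends the request and team name, sends the history, stores replies and exposes LatestMessage, including a generating placeholder.
; A separate Test event looks up M_CyberPiazza in DT_MapsData to set MapDetails.
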(event `self.ReceiveBeginPlay`
  (`self.InitializeGptAgent`))

(event `Test`
  (bind _returnvalue (`|GetDataTableRow` "/Game/Blueprints/MenusLogic/DT_MapsData.DT_MapsData" "M_CyberPiazza")
    (:`then`
      (set `self.MapDetails` _returnvalue))))

(event `InitializeGptAgent`
  (bind (_name _image _imageurl _areasbycolormap) (break `/Game/Blueprints/MenusLogic/S_MapDetails` (`self.MapDetails`)))
  (bind _promptmessage (`self.GenerateMapZonesByColor` _areasbycolormap))
  (`HttpGPTSettings.SetChatOptions` (make `HttpGPTChatOptions` "gpt35turbo"))
  (`HttpGPTSettings.SetCommonOptions` (make `HttpGPTCommonOptions` (`KismetStringLibrary.Conv_StringToName` (`self.GPT_KEY`))))
  (set `self.Messages` (`|MakeArray` (make `HttpGPTChatMessage` "System" (`KismetStringLibrary.Concat_StrStr` "You are a generator of team tactics for a shooter video game. Each team has 5 members and the goal is to eliminate the other team members." "The overview of the map which you have to analyze can be found at this URL:" _imageurl _promptmessage)) (make `HttpGPTChatMessage` "User" "Send your responses in a single block of text please, and keep them at max 300 words. When giving the answer, always mention what each team member will do. Use spaces for alignments and don't use ** for bold text.") (make `HttpGPTChatMessage` "Assistant" "Ok, I am ready."))))

(event `SendGptMessage`
  (params (MessageContent :type String) (TeamName :type String))
  (`KismetArrayLibrary.Array_Add` (`self.Messages`) (make `HttpGPTChatMessage` "User" (`KismetStringLibrary.Concat_StrStr` MessageContent " I am in " TeamName ".")))
  (bind (_asynctaskproxy _response) (`HttpGPTChatRequest.SendMessages_CustomOptions` :`Messages` (`self.Messages`) :`CommonOptions` (make `HttpGPTCommonOptions` (`KismetStringLibrary.Conv_StringToName` (`self.GPT_KEY`))) :`ChatOptions` (make `HttpGPTChatOptions` "gpt35turbo"))
    (:`ProcessCompleted`
      (bind (_index _message) (break `HttpGPTChatChoice` (`|GetArrayItem` (`.Choices` (break `HttpGPTChatResponse` _response)))))
      (`KismetArrayLibrary.Array_Add` (`self.Messages`) _message)
      (set `self.LatestMessage` (`.Content` (break `HttpGPTChatMessage` _message))))
    (:`ProgressStarted`
      (set `self.LatestMessage` "Generating..." :!label _label))
    (:`ErrorReceived`
      (`KismetSystemLibrary.PrintString` "GPT Error" :!label _label_2))
    (:`RequestFailed`
      (goto _label_2))
    (:`RequestSent`
      (goto _label))))

(fn `GenerateMapZonesByColor`
  (params (TargetMap :type "Map of String to String (by ref)"))
  (returns (PromptMessage :type String))
  (locals (MessagePrompt :type String :default "The map will always be splitted into zones which are color coded. For the map at the URL provided, we have the following zones associated with colors: "))
  (bind _keys (`BlueprintMapLibrary.Map_Keys` TargetMap))
  (for _array_element _keys
    (set `local.MessagePrompt` (`KismetStringLibrary.Concat_StrStr` (`local.MessagePrompt`) "Color: " _array_element "-> Zone Name: " (`BlueprintMapLibrary.Map_Find` TargetMap _array_element))))
  (return (`local.MessagePrompt`)))

(fn `UserConstructionScript`)