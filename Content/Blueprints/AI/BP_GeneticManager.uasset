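; Genetic algorithm manager that evolves recoil, jumpiness and fire-rate genes for red and blue AI bot teams over timed generations.
; SpawnGeneration seeds bots randomly or from saved genes initially, then from crossover and mutation of random parents.
; Rounds end on timeout or few survivors, then weighted fitness (accuracy, survival, kills, jumping) filters out zero scores.
; SaveGenesValues reads the just-cleared new-generation array; LoadGenerationData is never called here; HUD creation is unwired.
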(event `SpawnGeneration`
  (bind _botsarray (`self.BotsArray`))
  (bind _botsarray_2 (`self.BotsArray`))
  (bind _spawnvolume (`self.SpawnVolume`))
  ;[1 1 1] Spawn a generation
  (`/Engine/EditorBlueprintResources/StandardMacros.IncrementInt` (`self.CurrentGeneration`)
    (:`  `
      (for _index (range (+ (`self.BotsPerGeneration`) 1))
        ;;[1 0.9865 0.6908] Spawn in world
        (if (<= _index 4)
          (set `self.BotType` "/Game/Blueprints/AI/BP_Bot_Blue.BP_Bot_Blue_C")
          (else
            (set `self.BotType` "/Game/Blueprints/AI/BP_Bot_Red.BP_Bot_Red_C")))
        (bind _returnvalue (`AIBlueprintHelperLibrary.SpawnAIFromClass` (`self.BotType`) "/Game/Blueprints/AI/BT_Bot.BT_Bot" (`KismetMathLibrary.RandomPointInBoundingBox` (`SceneComponent.K2_GetComponentLocation` _spawnvolume) (`BoxComponent.GetScaledBoxExtent` _spawnvolume)) (`KismetMathLibrary.MakeRotator` 0.0 0.0 (`KismetMathLibrary.RandomFloatInRange` 0.0 360.0)) false null))
        (bind _asbp_bot (cast `/Game/Blueprints/AI/BP_Bot` _returnvalue))
        (set `self.BotSpawned` _asbp_bot)
        (set `/Game/Blueprints/AI/BP_Bot.Spawner` self (`self.BotSpawned`))
        (if (<= _index 4)
          (set `/Game/Blueprints/AI/BP_Bot.TeamTag` (struct :`TagName` "Team.BlueTeam") (`self.BotSpawned`))
          (else
            (set `/Game/Blueprints/AI/BP_Bot.TeamTag` (struct :`TagName` "Team.RedTeam") (`self.BotSpawned`))))
        (if (`self.IsFirstGenerationSpawned`)
          (if (<= (`self.CurrentGeneration`) 1)
            ;;[0.5349 0.7361 1] Spawn random values for first generation
            (`/Game/Blueprints/AI/BP_Bot.ConstructorInput` (`self.BotSpawned`) (make `/Game/Blueprints/AI/S_MutableGenes` (`KismetMathLibrary.RandomFloatInRange` (`self.Min_MinRecoil`) (`self.Max_MinRecoil`)) (`KismetMathLibrary.RandomFloatInRange` (`self.Min_MaxRecoil`) (`self.Max_MaxRecoil`)) (`KismetMathLibrary.RandomFloatInRange` (`self.Min_Jumpiness`) (`self.Max_Jumpiness`)) (`KismetMathLibrary.RandomFloatInRange` (`self.Min_FireRate`) (`self.Max_FireRate`))))
            (else
              ;;[1 1 1] Get genes values from saved data
              (bind (_minrecoil _maxrecoil _jumpiness _firerate) (`self.LoadGenesValues`))
              (`/Game/Blueprints/AI/BP_Bot.ConstructorInput` (`self.BotSpawned`) (make `/Game/Blueprints/AI/S_MutableGenes` _minrecoil _maxrecoil _jumpiness _firerate))))
          (else
            ;;[0.6354 1 1] Spawn gene values from crossover for next generations
            (bind _newgenes (`self.Crossover` (`KismetArrayLibrary.Array_Random` _botsarray) (`KismetArrayLibrary.Array_Random` _botsarray)))
            (`/Game/Blueprints/AI/BP_Bot.ConstructorInput` (`self.BotSpawned`) _newgenes)))
        (`KismetArrayLibrary.Array_Add` (`self.BotsArrayNewGen`) (`self.BotSpawned`)))
      ;;[1 0.7924 0.7322] Clear arrays and old generation
      (set `self.IsFirstGenerationSpawned` false)
      (for _array_element _botsarray_2
        (`self.SetLifeSpan` _array_element 0.1))
      (`KismetArrayLibrary.Array_Clear` _botsarray_2)
      (set `self.BotsArray` (`self.BotsArrayNewGen`))
      (`KismetArrayLibrary.Array_Clear` (`self.BotsArrayNewGen`))
      (`/Game/Blueprints/AI/UI/W_GeneticHUD.PopulateBox` (`self.Genetic_HUD`))
      ;;[1 1 1] Set timer for generation lifespan (how much a generation will live)
      (bind _returnvalue_2 (`KismetSystemLibrary.K2_SetTimer` null "EvaluateGenerationByFitness" (`self.MaxSurvivalTime`)))
      (set `self.GenerationRoundDurationHandler` _returnvalue_2))))

(event `self.ReceiveBeginPlay`
  ;[1 1 1] Create UI and start first generation
  (`self.SpawnGeneration`))

(event `RemoveIndividual`
  (params (KillerBot :type "/Game/Blueprints/AI/BP_Bot Object Reference"))
  ;[1 1 1] Method when an individual is eliminated
  (`/Engine/EditorBlueprintResources/StandardMacros.IncrementInt` (`/Game/Blueprints/AI/BP_Bot.NumberOfKills` KillerBot)
    (:`  `
      (set `self.NumberOfDeads` 1)
      (for _array_element (`self.BotsArray`)
        (if (`/Game/Blueprints/AI/BP_Bot.Dead` _array_element)
          (`/Engine/EditorBlueprintResources/StandardMacros.IncrementInt` (`self.NumberOfDeads`))))
      (`KismetSystemLibrary.K2_SetTimer` null "CheckRoundFinish" 0.5))))

(fn `CheckRoundFinish`
  (locals (RemainingTeams :type "Set of GameplayTag Structure"))
  (bind _botsarray (`self.BotsArray`))
  (for _array_element _botsarray
    (`BlueprintSetLibrary.Set_Add` (`local.RemainingTeams`) (`/Game/Blueprints/AI/BP_Bot.TeamTag` _array_element)))
  (if (or (<= (- (`KismetArrayLibrary.Array_Length` _botsarray) (`self.NumberOfDeads`)) 2) (== (`BlueprintSetLibrary.Set_Length` (`local.RemainingTeams`)) 1))
    (`self.EvaluateGenerationByFitness`)))

(fn `Crossover`
  (params (Parent1 :type "/Game/Blueprints/AI/BP_Bot Object Reference") (Parent2 :type "/Game/Blueprints/AI/BP_Bot Object Reference"))
  (returns (NewGenes :type "/Game/Blueprints/AI/S_MutableGenes Structure"))
  (locals (MutableGenes :type "/Game/Blueprints/AI/S_MutableGenes Structure") (P1 :type "/Game/Blueprints/AI/BP_Bot Object Reference") (P2 :type "/Game/Blueprints/AI/BP_Bot Object Reference"))
  (set `local.P1` Parent1)
  (set `local.P2` Parent2)
  (bind _output_get (set `local.MutableGenes` (make `/Game/Blueprints/AI/S_MutableGenes` (`KismetMathLibrary.FMax` (`/Game/Blueprints/AI/BP_Bot.MinRecoil` (`local.P1`)) (`/Game/Blueprints/AI/BP_Bot.MinRecoil` (`local.P2`))) (`KismetMathLibrary.FMin` (`/Game/Blueprints/AI/BP_Bot.MaxRecoil` (`local.P1`)) (`/Game/Blueprints/AI/BP_Bot.MaxRecoil` (`local.P2`))) (`KismetMathLibrary.FMin` (`/Game/Blueprints/AI/BP_Bot.JumpingResultValue` (`local.P1`)) (`/Game/Blueprints/AI/BP_Bot.JumpingResultValue` (`local.P2`))) (`KismetMathLibrary.FMax` (`/Game/Blueprints/AI/BP_Bot.FireRate` (`local.P1`)) (`/Game/Blueprints/AI/BP_Bot.FireRate` (`local.P2`))))))
  (bind _genes (`self.Mutate` _output_get))
  (return _genes))

(fn `EvaluateGenerationByFitness`
  (`KismetSystemLibrary.K2_ClearAndInvalidateTimerHandle` (`self.GenerationRoundDurationHandler`))
  (for _array_element (`self.BotsArray`)
    ;[1 1 1] Filter bots with 0 fitness score
    (bind _score (`self.FitnessFunction` _array_element))
    (bind _output_get (set `/Game/Blueprints/AI/BP_Bot.FitnessScore` _score _array_element))
    (if (!= _output_get 0.0)
      (`KismetArrayLibrary.Array_Add` (`self.BotsArrayNewGen`) _array_element)))
  ;[1 1 1] BotsArray should contain filtered individuals with fitnessScore > 0 and NewGen array should be empty
  (`KismetArrayLibrary.Array_Clear` (`self.BotsArray`))
  (set `self.BotsArray` (`self.BotsArrayNewGen`))
  (`KismetArrayLibrary.Array_Clear` (`self.BotsArrayNewGen`))
  (`self.SaveGenesValues`)
  ;[1 1 1] Spawn new generation
  (`KismetSystemLibrary.K2_SetTimer` null "SpawnGeneration" 15.0))

(fn `FitnessFunction`
  (params (BotRef :type "/Game/Blueprints/AI/BP_Bot Object Reference"))
  (returns (Score :type "Float (double-precision)"))
  (locals (FinalScore :type "Float (double-precision)") (Bot :type "/Game/Blueprints/AI/BP_Bot Object Reference") (AccuracyScore :type "Float (double-precision)") (SurvivalTimeScore :type "Float (double-precision)") (KillsNumberScore :type "Float (double-precision)") (JumpingScore :type "Float (double-precision)") (AccuracyWeight :type "Float (double-precision)" :default 0.2) (SurvivalTimeWeight :type "Float (double-precision)" :default 0.2) (KillsNumberWeight :type "Float (double-precision)" :default 0.5) (JumpingWeight :type "Float (double-precision)" :default 0.1))
  (bind _survivaltime (`/Game/Blueprints/AI/BP_Bot.SurvivalTime` (`local.Bot`)))
  (set `local.Bot` BotRef)
  (if (and (<= _survivaltime (`self.MinSurvivalTime`)) (!= _survivaltime -1.0))
    (return 0.0)
    (else
      ;[1 1 1] Calculate each gene's score
      (set `local.SurvivalTimeScore` (/ _survivaltime (`self.MaxSurvivalTime`)))
      (set `local.AccuracyScore` (/ (`KismetMathLibrary.Conv_IntToDouble` (`/Game/Blueprints/AI/BP_Bot.NumberOfHits` (`local.Bot`))) (`KismetMathLibrary.Conv_IntToDouble` (`/Game/Blueprints/AI/BP_Bot.NumberOfShotsFired` (`local.Bot`)))))
      (set `local.JumpingScore` (`/Game/Blueprints/AI/BP_Bot.JumpingResultValue` (`local.Bot`)))
      (set `local.KillsNumberScore` (`KismetMathLibrary.Conv_IntToDouble` (`/Game/Blueprints/AI/BP_Bot.NumberOfKills` (`local.Bot`))))
      (bind _output_get (set `local.FinalScore` (+ (* (`local.AccuracyScore`) (`local.AccuracyWeight`)) (* (`local.SurvivalTimeScore`) (`local.SurvivalTimeWeight`)) (* (`local.KillsNumberScore`) (`local.KillsNumberWeight`)) (* (`local.JumpingScore`) (`local.JumpingWeight`)))))
      (return _output_get))))

(fn `LoadGenerationData`
  (bind _returnvalue (`GameplayStatics.DoesSaveGameExist` (`self.SaveGameSlot`)))
  (if _returnvalue
    (bind _returnvalue_2 (`GameplayStatics.LoadGameFromSlot` (`self.SaveGameSlot`)))
    (bind _asbp_save_game_ai (cast `/Game/Blueprints/AI/SaveGame/BP_SaveGameAI` _returnvalue_2))
    (bind _output_get (set `self.SavedGameData` _asbp_save_game_ai))
    (set `self.CurrentGeneration` (`/Game/Blueprints/AI/SaveGame/BP_SaveGameAI.CurrentGeneration` _output_get))))

(fn `LoadGenesValues`
  (returns (MinRecoil :type "Float (double-precision)") (MaxRecoil :type "Float (double-precision)") (Jumpiness :type "Float (double-precision)") (FireRate :type "Float (double-precision)"))
  (bind _savedgamedata (`self.SavedGameData`)
    (:`then`
      (return (`/Game/Blueprints/AI/SaveGame/BP_SaveGameAI.MinRecoil` _savedgamedata) (`/Game/Blueprints/AI/SaveGame/BP_SaveGameAI.MaxRecoil` _savedgamedata) (`/Game/Blueprints/AI/SaveGame/BP_SaveGameAI.Jumpiness` _savedgamedata) (`/Game/Blueprints/AI/SaveGame/BP_SaveGameAI.FireRate` _savedgamedata)))
    (:`else`)))

(fn `Mutate`
  (params (NewGenes :type "/Game/Blueprints/AI/S_MutableGenes Structure"))
  (returns (Genes :type "/Game/Blueprints/AI/S_MutableGenes Structure"))
  (locals (MutatedMinRecoil :type "Float (double-precision)" :default 0.0) (MutatedMaxRecoil :type "Float (double-precision)" :default 0.0) (MutatedJumpiness :type "Float (double-precision)" :default 0.0) (MutatedFireRate :type "Float (double-precision)" :default 0.0))
  (bind _shouldmutate (`self.ShouldMutate` 0.4))
  (if _shouldmutate
    (set `local.MutatedMinRecoil` (`KismetMathLibrary.FClamp` (+ (`KismetMathLibrary.RandomFloatInRange` 0.0 1.0) NewGenes_MinRecoil_2_1C6F80434D10F1203E8157BDCA3CDAA7) (`self.Min_MinRecoil`) (`self.Max_MinRecoil`)))
    (else
      (set `local.MutatedMinRecoil` NewGenes_MinRecoil_2_1C6F80434D10F1203E8157BDCA3CDAA7)))
  (bind _shouldmutate_2 (`self.ShouldMutate` 0.4))
  (if _shouldmutate_2
    (set `local.MutatedMaxRecoil` (`KismetMathLibrary.FClamp` (+ (`KismetMathLibrary.RandomFloatInRange` 0.0 -1.0) NewGenes_MaxRecoil_4_DDBC8E8C4A783FB00E5ACAB45A0A008F) (`self.Min_MaxRecoil`) (`self.Max_MaxRecoil`)))
    (else
      (set `local.MutatedMaxRecoil` NewGenes_MaxRecoil_4_DDBC8E8C4A783FB00E5ACAB45A0A008F)))
  (bind _shouldmutate_3 (`self.ShouldMutate` 0.4))
  (if _shouldmutate_3
    (set `local.MutatedJumpiness` (`KismetMathLibrary.FClamp` (+ (`KismetMathLibrary.RandomFloatInRange` 0.0 1.0) NewGenes_Jumpiness_6_7A8C156846D1433A8394A2952B449591) 0.0 (`self.Max_Jumpiness`)))
    (else
      (set `local.MutatedJumpiness` NewGenes_Jumpiness_6_7A8C156846D1433A8394A2952B449591)))
  (bind _shouldmutate_4 (`self.ShouldMutate` 0.3))
  (if _shouldmutate_4
    (set `local.MutatedFireRate` (`KismetMathLibrary.FClamp` (+ (`KismetMathLibrary.RandomFloatInRange` 0.5) NewGenes_FireRate_8_09C058F045CB6F48AC87FEB484F26668)))
    (else
      (set `local.MutatedFireRate` NewGenes_FireRate_8_09C058F045CB6F48AC87FEB484F26668)))
  (return (make `/Game/Blueprints/AI/S_MutableGenes` (`local.MutatedMinRecoil`) (`local.MutatedMaxRecoil`) (`local.MutatedJumpiness`) (`local.MutatedFireRate`))))

(fn `SaveGenesValues`
  (bind _output (`|GetArrayItem` (`self.BotsArrayNewGen`)))
  (bind _returnvalue (`GameplayStatics.CreateSaveGameObject` "/Game/Blueprints/AI/SaveGame/BP_SaveGameAI.BP_SaveGameAI_C"))
  (set `/Game/Blueprints/AI/SaveGame/BP_SaveGameAI.MinRecoil` (`/Game/Blueprints/AI/BP_Bot.MinRecoil` _output) _returnvalue)
  (set `/Game/Blueprints/AI/SaveGame/BP_SaveGameAI.MaxRecoil` 0.0 _returnvalue)
  (set `/Game/Blueprints/AI/SaveGame/BP_SaveGameAI.Jumpiness` (`/Game/Blueprints/AI/BP_Bot.MinJumpiness` _output) _returnvalue)
  (set `/Game/Blueprints/AI/SaveGame/BP_SaveGameAI.FireRate` (`/Game/Blueprints/AI/BP_Bot.FireRate` _output) _returnvalue)
  (set `/Game/Blueprints/AI/SaveGame/BP_SaveGameAI.CurrentGeneration` (`self.CurrentGeneration`) _returnvalue)
  (`GameplayStatics.SaveGameToSlot` _returnvalue (`self.SaveGameSlot`)))

(fn `ShouldMutate`
  (params (MutationRate :type "Float (double-precision)"))
  (returns (ShouldMutate :type Boolean))
  (return (<= (`KismetMathLibrary.RandomFloatInRange` 0.0 1.0) MutationRate)))

(fn `UserConstructionScript`)